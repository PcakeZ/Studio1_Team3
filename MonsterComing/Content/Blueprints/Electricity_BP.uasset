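; Electricity_BP is a timed electric hazard actor that electrocutes the player character on contact.
; On BeginPlay it unhides its Electricity and PreElectricty components, enables Sphere collision after a short delay, then destroys itself once a longer delay ends.
; When a ThirdPersonCharacter begins overlapping the Sphere, it calls DebuffElectrocuted on player 0's character rather than on the overlapping actor.
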(event OnComponentBeginOverlap(Sphere)
  (params (OverlappedComponent :type Primitive%20Component%20Object%20Reference) (OtherActor :type Actor%20Object%20Reference) (OtherComp :type Primitive%20Component%20Object%20Reference) (OtherBodyIndex :type Integer) (bFromSweep :type Boolean) (SweepResult :type Hit%20Result%20Structure%20%28by%20ref%29))
  (if (== (Utilities|GetClass OtherActor) "/Game/Assets/Blueprints/Player_Blueprints/ThirdPersonCharacter.ThirdPersonCharacter_C")
    (bind _asthird_person_character (Utilities|Casting|CastToThirdPersonCharacter (Game|GetPlayerCharacter 0)))
    (Default|Debuff:Electrocuted _asthird_person_character)))

(event EventBeginPlay
  (Development|SetHiddeninGame (Variables|Default|GetElectricity) false false)
  (Development|SetHiddeninGame (Variables|Default|GetPreElectricty) false false)
  (Utilities|FlowControl|Delay 1.0)
  (Collision|SetCollisionEnabled (Variables|Default|GetSphere) "QueryAndPhysics")
  (Utilities|FlowControl|Delay 1e+01)
  (Actor|DestroyActor))

(event Collision|EventActorBeginOverlap
  (params (OtherActor :type Actor%20Object%20Reference)))

(event EventTick
  (params (DeltaSeconds :type Float%20%28single-precision%29)))

(fn ConstructionScript)