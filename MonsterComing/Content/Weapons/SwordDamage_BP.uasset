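; SwordDamage_BP is a weapon Blueprint that animates a pin mesh, with no damage logic in its graphs.
; On BeginPlay it adds to MyFpsGears and caches the ThirdPersonGameMode.
; Each Tick, RotatePin composes a sine-driven yaw from game time onto MeterCylinder001's current world transform, so the wobble accumulates per frame rather than setting an absolute angle.
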(event EventBeginPlay
  (Utilities|Array|Add (Variables|Default|GetMy_FpsGears) 0)
  (bind _asthird_person_game_mode (Utilities|Casting|CastToThirdPersonGameMode (Game|GetGameMode)))
  (Variables|Default|SetGamemode _asthird_person_game_mode))

(event Collision|EventActorBeginOverlap
  (params (OtherActor :type Actor%20Object%20Reference)))

(event EventTick
  (params (DeltaSeconds :type Float%20%28single-precision%29))
  (CallFunction|RotatePin (Utilities|Time|GetGameTimeinSeconds)))

(fn ConstructionScript)

(fn RotatePin
  (params (Time :type Float%20%28single-precision%29))
  (bind _meter_cylinder_001 (Variables|Default|GetMeter_Cylinder_001))
  (Transformation|SetWorldTransform _meter_cylinder_001 (Math|Transform|ComposeTransforms (Math|Transform|MakeTransform "0, 0, 0" (Math|Rotator|MakeRotator 0.0 0.0 (* (Math|Trig|Sin(Radians) (* Time 2e+01)) 1e+01))) (Transformation|GetWorldTransform _meter_cylinder_001)) false false))