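; Sword actor that animates decorative gears and a meter cylinder on its model.
; Each Tick, it spins five gear components by fixed yaw steps in alternating or matched directions, and oscillates the cylinder with a sine of game time.
; Rotations compose onto current transforms in local space without delta-time scaling, so motion depends on frame rate.
; BeginPlay also caches the ThirdPersonGameMode, which nothing here reads.
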(event EventBeginPlay
  (Utilities|Array|Add (Variables|Default|GetMy_FpsGears) 0)
  (bind _asthird_person_game_mode (Utilities|Casting|CastToThirdPersonGameMode (Game|GetGameMode)))
  (Variables|Default|SetGamemode _asthird_person_game_mode))

(event Collision|EventActorBeginOverlap
  (params (OtherActor :type Actor%20Object%20Reference)))

(event EventTick
  (params (DeltaSeconds :type Float%20%28single-precision%29))
  (for (_array_element _array_index) (Utilities|Array|MakeArray (Variables|Default|GetSwordGears2_Meter_003) (Variables|Default|GetSwordGears2_Meter_001) (Variables|Default|GetSwordGears2_Meter_004) (Variables|Default|GetSwordGears2_Meter_005) (Variables|Default|GetSwordGears2_Meter_002))
    (CallFunction|RotateGears _array_element _array_index _array_element _array_element _array_element _array_element))
  (CallFunction|RotatePin (Utilities|Time|GetGameTimeinSeconds)))

(fn ConstructionScript)

(fn RotateGear
  (params (Rotation :type Float%20%28single-precision%29) (GearToRotate :type Static%20Mesh%20Component%20Object%20Reference))
  (Transformation|SetWorldTransform GearToRotate (Math|Transform|ComposeTransforms (Math|Transform|MakeTransform "0, 0, 0" (Math|Rotator|MakeRotator 0.0 0.0 Rotation)) (Transformation|GetWorldTransform GearToRotate)) false false))

(fn RotateGears
  (params (GearToRotate :type Static%20Mesh%20Component%20Object%20Reference) (Selection :type Integer) (GearToRotate2 :type Static%20Mesh%20Component%20Object%20Reference) (GearToRotate3 :type Static%20Mesh%20Component%20Object%20Reference) (GearToRotate4 :type Static%20Mesh%20Component%20Object%20Reference) (GearToRotate5 :type Static%20Mesh%20Component%20Object%20Reference))
  (switch int Selection
    (:0
      (CallFunction|RotateGear 3.0 GearToRotate2))
    (:1
      (CallFunction|RotateGear -2.0 GearToRotate))
    (:2
      (CallFunction|RotateGear 3.0 GearToRotate5))
    (:3
      (CallFunction|RotateGear -2.0 GearToRotate4))
    (:4
      (CallFunction|RotateGear -2.0 GearToRotate3))))

(fn RotatePin
  (params (Time :type Float%20%28single-precision%29))
  (bind _meter_cylinder_001 (Variables|Default|GetMeter_Cylinder_001))
  (Transformation|SetWorldTransform _meter_cylinder_001 (Math|Transform|ComposeTransforms (Math|Transform|MakeTransform "0, 0, 0" (Math|Rotator|MakeRotator 0.0 0.0 (* (Math|Trig|Sin(Radians) (* Time 2e+01)) 1e+01))) (Transformation|GetWorldTransform _meter_cylinder_001)) false false))