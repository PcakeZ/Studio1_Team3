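; Upgrade machine that opens the turret upgrade UI for the player.
; Overlap tracks the character; the Upgrade1M event, while colliding, disables movement, flags machine contact and sets the game mode's widget to TurretUpgradeUI.
; Ending overlap restores movement, clears the flag and switches back to InGameUI.
; An unconnected chain would draw the weapon if needed, then spawn an anvil spark effect after a delay.
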(event Custom|Upgrade1M
  (bind _player_character (Variables|Default|GetPlayer%20Character))
  (if (Variables|Default|GetCollide)
    (Variables|/Game/Assets/Blueprints/Player_Blueprints/ThirdPersonCharacter.ThirdPersonCharacter_C|SetCanMove _player_character false)
    (Variables|/Game/Assets/Blueprints/Player_Blueprints/ThirdPersonCharacter.ThirdPersonCharacter_C|SetisMachineColl _player_character true)
    (bind _asthird_person_game_mode (Utilities|Casting|CastToThirdPersonGameMode (Game|GetGameMode)))
    (Variables|/Game/Assets/Blueprints/GameMode/ThirdPersonGameMode.ThirdPersonGameMode_C|SetNewWidget _asthird_person_game_mode "TurretUpgradeUI")))

(event Collision|EventActorBeginOverlap
  (params (OtherActor :type Actor%20Object%20Reference))
  (bind _asthird_person_character (Utilities|Casting|CastToThirdPersonCharacter OtherActor))
  (Variables|Default|SetCollide true)
  (bind _output_get (Variables|Default|SetPlayer%20Character _asthird_person_character)))

(event Collision|EventActorEndOverlap
  (params (OtherActor :type Actor%20Object%20Reference))
  (bind _asthird_person_character (Utilities|Casting|CastToThirdPersonCharacter OtherActor))
  (Variables|/Game/Assets/Blueprints/Player_Blueprints/ThirdPersonCharacter.ThirdPersonCharacter_C|SetCanMove _asthird_person_character true)
  (Variables|/Game/Assets/Blueprints/Player_Blueprints/ThirdPersonCharacter.ThirdPersonCharacter_C|SetisMachineColl _asthird_person_character false)
  (Variables|Default|SetCollide false)
  (bind _asthird_person_game_mode (Utilities|Casting|CastToThirdPersonGameMode (Game|GetGameMode)))
  (Variables|/Game/Assets/Blueprints/GameMode/ThirdPersonGameMode.ThirdPersonGameMode_C|SetNewWidget _asthird_person_game_mode "InGameUI"))

(fn ConstructionScript)