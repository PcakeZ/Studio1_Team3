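; Anvil actor that performs a weapon upgrade, swapping the player's Weapon2 for Weapon3.
; Overlap events cache the ThirdPersonCharacter and toggle its IsAnvilColl flag, which gates the Upgrade2 event.
; Upgrade2 draws the weapon if needed, waits, spawns an explosion effect, swaps mesh visibility and plays an inspect montage.
; It disables CanMove during the montage and sets it false again after the delay, so movement is never restored here.
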(event Custom|Upgrade2
  (bind _player_character (Variables|Default|GetPlayer%20Character))
  (bind _player_character_2 (Variables|Default|GetPlayer%20Character))
  (bind _player_character_3 (Variables|Default|GetPlayer%20Character))
  (Utilities|IsValid (stale Collision|EventActorBeginOverlap _output_get)
    (:Is%20Valid
      (if (Variables|/Game/Assets/Blueprints/Player_Blueprints/ThirdPersonCharacter.ThirdPersonCharacter_C|GetisAnvilColl (Variables|Default|GetPlayer%20Character))
        (Development|PrintString "upg2")
        ;[1 1 1] sparks come out of anvil
        (if (Variables|/Game/Assets/Blueprints/Player_Blueprints/ThirdPersonCharacter.ThirdPersonCharacter_C|GetWeaponDrawn _player_character_3)
          (Utilities|FlowControl|Delay 0.2)
          (else
            ;;[1 1 1] equip weapon if not drawn
            (Default|DrawWeapon _player_character_3)
            (Utilities|FlowControl|Delay 1.3)))
        (Effects|SpawnEmitterAttached "/Game/StarterContent/Particles/P_Explosion.P_Explosion" (Variables|Default|GetParticleSystem) "None" "0, 0, 0" "0, 0, 0" "5.000000,5.000000,5.000000")
        ;[1 1 1] Set upgraded weapon visibility
        (Rendering|SetVisibility (Variables|/Game/Assets/Blueprints/Player_Blueprints/ThirdPersonCharacter.ThirdPersonCharacter_C|GetWeapon2 _player_character_2) false false)
        (Rendering|SetVisibility (Variables|/Game/Assets/Blueprints/Player_Blueprints/ThirdPersonCharacter.ThirdPersonCharacter_C|GetWeapon3 _player_character_2) true false)
        (Animation|Montage|PlayMontage (Variables|/Script/Engine.Character|GetMesh (Variables|Default|GetPlayer%20Character)) "/Game/Mannequin/Animations/InspectWeapon_Montage.InspectWeapon_Montage"
          (:then
            ;[1 1 1] Pause movement
            (Variables|/Game/Assets/Blueprints/Player_Blueprints/ThirdPersonCharacter.ThirdPersonCharacter_C|SetCanMove _player_character false)
            (Utilities|FlowControl|Delay 5.0)
            (Variables|/Game/Assets/Blueprints/Player_Blueprints/ThirdPersonCharacter.ThirdPersonCharacter_C|SetCanMove _player_character false)))))))

(event Collision|EventActorBeginOverlap
  (params (OtherActor :type Actor%20Object%20Reference))
  (bind _asthird_person_character (Utilities|Casting|CastToThirdPersonCharacter OtherActor))
  (bind _output_get (Variables|Default|SetPlayer%20Character _asthird_person_character))
  (Variables|/Game/Assets/Blueprints/Player_Blueprints/ThirdPersonCharacter.ThirdPersonCharacter_C|SetisAnvilColl _output_get true)
  (Development|PrintString "overlap"))

(event Collision|EventActorEndOverlap
  (params (OtherActor :type Actor%20Object%20Reference))
  (bind _asthird_person_character (Utilities|Casting|CastToThirdPersonCharacter OtherActor))
  (Variables|/Game/Assets/Blueprints/Player_Blueprints/ThirdPersonCharacter.ThirdPersonCharacter_C|SetisAnvilColl _asthird_person_character false)
  (Development|PrintString "not overlap"))

(fn ConstructionScript)