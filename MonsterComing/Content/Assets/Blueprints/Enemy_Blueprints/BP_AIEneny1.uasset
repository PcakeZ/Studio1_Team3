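; Enemy AI character that chases the player, switches to turrets it bumps into, and reverts to the player when the overlap ends.
; Tick drives AIMoveTo, the camera-facing health bar and an attack cooldown; successful moves trigger death or an in-range attack.
; Attack subtracts health directly from the player or turret.
; Incoming damage plays a hit reaction and subtracts the player's SwordDamage, ignoring hits while an animation plays.
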(event OnComponentBeginOverlap(CapsuleComponent)
  (params (OverlappedComponent :type Primitive%20Component%20Object%20Reference) (OtherActor :type Actor%20Object%20Reference) (OtherComp :type Primitive%20Component%20Object%20Reference) (OtherBodyIndex :type Integer) (bFromSweep :type Boolean) (SweepResult :type Hit%20Result%20Structure%20%28by%20ref%29))
  ;[1 1 1] If player collides with turret, set turret as current taget
  (Utilities|Casting|CastToThirdPersonCharacter OtherActor
    (:CastFailed
      (bind _asbp_turret (Utilities|Casting|CastToBP_Turret OtherActor))
      (if (not (== (Variables|/Game/Assets/Blueprints/Turret_Blueprints/BP_Turret.BP_Turret_C|GetAttackRadius _asbp_turret) OtherComp))
        (Variables|Default|SetTargetActor _asbp_turret)
        (Development|PrintString "Turret is target")))))

(event OnComponentEndOverlap(CapsuleComponent)
  (params (OverlappedComponent :type Primitive%20Component%20Object%20Reference) (OtherActor :type Actor%20Object%20Reference) (OtherComp :type Primitive%20Component%20Object%20Reference) (OtherBodyIndex :type Integer))
  ;[1 1 1] If ai stops collision with the turret, set target to player
  (Utilities|Casting|CastToBP_Turret OtherActor)
  (bind _outactors (Actor|GetAllActorsOfClass "/Game/Assets/Blueprints/Player_Blueprints/ThirdPersonCharacter.ThirdPersonCharacter_C"))
  (Variables|Default|SetTargetActor (Utilities|Array|Get(acopy) _outactors)))

(event EventTick
  (params (DeltaSeconds :type Float%20%28single-precision%29))
  (bind _widget (Variables|Default|GetWidget))
  (bind _healthbar (Variables|Default|GetHealthbar))
  ;[1 1 1] Set Values
  (Variables|/Script/Engine.CharacterMovementComponent|SetMaxWalkSpeed (Variables|Character|GetCharacterMovement) (Variables|Default|GetMovementSpeed))
  (Variables|Default|SetCurrentAttackSpeed (- (Variables|Default|GetCurrentAttackSpeed) DeltaSeconds))
  ;[1 1 1] HealthBar look at camera
  (bind _asthird_person_character (Utilities|Casting|CastToThirdPersonCharacter (Variables|Default|GetPlayer)))
  (Transformation|SetWorldRotation _widget (Math|Rotator|FindLookatRotation (Transformation|GetWorldLocation _widget) (Transformation|GetWorldLocation (Variables|/Game/Assets/Blueprints/Player_Blueprints/ThirdPersonCharacter.ThirdPersonCharacter_C|GetFollowCamera _asthird_person_character))) false false)
  ;[1 1 1] Set Healthbar percent to health
  (if (Utilities|IsValid _healthbar)
    (Variables|/Game/Assets/Widgets/AIHealthBar.AIHealthBar_C|SetHealthPercentage _healthbar (/ (Variables|Default|GetCurrentHealth) (Variables|Default|GetMaxHealth)))
    ;[1 1 1] Test if AI has a target
    (if (Utilities|IsValid (Variables|Default|GetTargetActor))
      ;[1 1 1] Move to taget
      (AI|AIMoveTo self "0, 0, 0" (Variables|Default|GetTargetActor) 5.0 false
        (:then
          ;[1 1 1] Test Health
          (if (> (Variables|Default|GetCurrentHealth) 0.0)
            (if (< (Math|Vector|Distance(Vector) (Transformation|GetActorLocation self) (Transformation|GetActorLocation (Variables|Default|GetTargetActor))) (Variables|Default|GetMinAttackDistance))
              ;[1 1 1] If so, attack taget
              (CallFunction|Attack))
            (else
              ;[1 1 1] AI is dead
              (Actor|DestroyActor)))))
      (else
        ;[1 1 1] If not, set target to player
        (bind _outactors (Actor|GetAllActorsOfClass "/Game/Assets/Blueprints/Player_Blueprints/ThirdPersonCharacter.ThirdPersonCharacter_C"))
        (Variables|Default|SetTargetActor (Utilities|Array|Get(acopy) _outactors))))))

(event Game|Damage|EventAnyDamage
  (params (Damage :type Float%20%28single-precision%29) (DamageType :type Damage%20Type%20Object%20Reference) (InstigatedBy :type Controller%20Object%20Reference) (DamageCauser :type Actor%20Object%20Reference))
  (if (not (Audio|Components|Audio|IsPlaying (Variables|Character|GetMesh)))
    (Components|Animation|PlayAnimation (Variables|Character|GetMesh) "/Game/Mannequin/Animations/HitReaction/HitReaction.HitReaction" false)
    (Development|PrintString (Utilities|String|ToString(Float) Damage))
    (Variables|Default|SetCurrentHealth (- (Variables|Default|GetCurrentHealth) (Variables|/Game/Assets/Blueprints/Player_Blueprints/ThirdPersonCharacter.ThirdPersonCharacter_C|GetSwordDamage (Variables|Default|GetPlayer%20Reference))))))

(event EventBeginPlay
  ;[1 1 1] Set inital target to player
  (bind _outactors (Actor|GetAllActorsOfClass "/Game/Assets/Blueprints/Player_Blueprints/ThirdPersonCharacter.ThirdPersonCharacter_C"))
  (bind _output_get (Variables|Default|SetTargetActor (Utilities|Array|Get(acopy) _outactors)))
  (Variables|Default|SetPlayer _output_get)
  (bind _asthird_person_character (Utilities|Casting|CastToThirdPersonCharacter (Game|GetPlayerCharacter 0)))
  ;[1 1 1] Set other values
  (Variables|Default|SetPlayer%20Reference _asthird_person_character)
  (Variables|Default|SetCurrentHealth (Variables|Default|GetMaxHealth))
  (Variables|Default|SetCurrentAttackSpeed (Variables|Default|GetAttackSpeed)))

(fn ConstructionScript)

(fn Attack
  (if (< (Variables|Default|GetCurrentAttackSpeed) 0.0)
    (bind _asthird_person_character (Utilities|Casting|CastToThirdPersonCharacter (Variables|Default|GetTargetActor))
      (:then
        (Variables|/Game/Assets/Blueprints/Player_Blueprints/ThirdPersonCharacter.ThirdPersonCharacter_C|SetCurrentHealth _asthird_person_character (- (Variables|/Game/Assets/Blueprints/Player_Blueprints/ThirdPersonCharacter.ThirdPersonCharacter_C|GetCurrentHealth _asthird_person_character) (Variables|Default|GetDamage)))
        (Development|PrintString "Player Attacked")
        (Variables|Default|SetCurrentAttackSpeed (Variables|Default|GetAttackSpeed))
        (return))
      (:CastFailed
        (bind _asbp_turret (Utilities|Casting|CastToBP_Turret (Variables|Default|GetTargetActor)))
        (Variables|/Game/Assets/Blueprints/Turret_Blueprints/BP_Turret.BP_Turret_C|SetCurrentHealth _asbp_turret (- (Variables|/Game/Assets/Blueprints/Turret_Blueprints/BP_Turret.BP_Turret_C|GetCurrentHealth _asbp_turret) (Variables|Default|GetDamage)))
        (Development|PrintString "Turret Attacked")
        (Variables|Default|SetCurrentAttackSpeed (Variables|Default|GetAttackSpeed))
        (return)))))