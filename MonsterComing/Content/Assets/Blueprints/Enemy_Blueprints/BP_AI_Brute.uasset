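; Brute enemy AI that hunts the active door drill, nearby turrets or the player, and destroys itself at zero health.
; Tick updates its camera-facing health bar, runs SetTarget on check and switch timers, then moves to the target.
; Attack plays a punch montage on a cooldown and subtracts health directly, also resetting drill repair time.
; Incoming damage adds player sword damage and is DoOnce-gated around a hit reaction.
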(event Custom|Recovered
  ;[1 1 1] Hit by sword
  (Utilities|FlowControl|DoOnce false) ; enters at Reset
)

(event EventTick
  (params (DeltaSeconds :type Float%20%28single-precision%29))
  (bind _widget (Variables|Default|GetWidget))
  ;[1 1 1] Test Health
  (if (> (Variables|Default|GetCurrentHealth) 0.0)
    ;[1 1 1] HealthBar look at camera
    (Transformation|SetWorldRotation _widget (Math|Rotator|FindLookatRotation (Transformation|GetWorldLocation _widget) (Transformation|GetWorldLocation (Variables|/Game/Assets/Blueprints/Player_Blueprints/ThirdPersonCharacter.ThirdPersonCharacter_C|GetFollowCamera (Variables|Default|GetPlayer)))) false false)
    ;[1 1 1] Set Values
    (Variables|/Script/Engine.CharacterMovementComponent|SetMaxWalkSpeed (Variables|Character|GetCharacterMovement) (Variables|Default|GetMovementSpeed))
    (Variables|Default|SetCurrentAttackSpeed (- (Variables|Default|GetCurrentAttackSpeed) (Utilities|Time|GetWorldDeltaSeconds)))
    ;[1 1 1] Set Healthbar percent to health
    (Variables|/Game/Assets/Widgets/AIHealthBar.AIHealthBar_C|SetHealthPercentage (Variables|Default|GetHealthbar) (/ (Variables|Default|GetCurrentHealth) (Variables|Default|GetMaxHealth)))
    (Utilities|IsValid (Variables|Default|GetDrill)
      (:Is%20Valid
        (CallFunction|SetTarget :!label _label)
        (Utilities|IsValid (Variables|Default|GetTargetActor)
          (:Is%20Valid
            _)
          (:Is%20Not%20Valid
            (Utilities|IsValid (Variables|Default|GetDrill)
              (:Is%20Valid
                (Variables|Default|SetTargetActor (Variables|Default|GetDrill)))
              (:Is%20Not%20Valid
                (Variables|Default|SetTargetActor (Variables|Default|GetPlayer))))))
        ;[1 1 1] Move to taget
        (AI|AIMoveTo self "0, 0, 0" (Variables|Default|GetTargetActor) 5.0 false
          (:then
            ;[1 1 1] Attacking
            (if (< (Math|Vector|Distance(Vector) (Transformation|GetActorLocation self) (Transformation|GetActorLocation (Variables|Default|GetTargetActor))) (Variables|Default|GetMinAttackDistance))
              (CallFunction|Attack)
              (elif (and (< (Math|Vector|Distance(Vector) (Transformation|GetActorLocation self) (Transformation|GetActorLocation (Variables|Default|GetTargetActor))) (* (Variables|Default|GetMinAttackDistance) 2.0)) (== (Variables|Default|GetTargetActor) (Variables|Default|GetDrill)))
                (CallFunction|Attack)
                (else
                  (Variables|Default|SetCurrentAttackSpeed (Variables|Default|GetAttackSpeed))))))))
      (:Is%20Not%20Valid
        ;[1 1 1] Set Drill value
        (bind _outactors (Actor|GetAllActorsOfClass "/Game/Assets/Blueprints/Door_Drll/Door_Drill.Door_Drill_C"))
        (for _array_element _outactors
          (if (Variables|/Game/Assets/Blueprints/Door_Drll/Door_Drill.Door_Drill_C|GetIsActive _array_element)
            (bind _output_get (Variables|Default|SetDrill _array_element))
            (Variables|Default|SetTargetActor _output_get)
            (goto _label)
            (else
              (goto _label))))))
    (else
      ;[1 1 1] AI is dead
      (Actor|DestroyActor))))

(event Game|Damage|EventAnyDamage
  (params (Damage :type Float%20%28single-precision%29) (DamageType :type Damage%20Type%20Object%20Reference) (InstigatedBy :type Controller%20Object%20Reference) (DamageCauser :type Actor%20Object%20Reference))
  ;[1 1 1] Hit by sword
  (Utilities|FlowControl|DoOnce false
    (:Completed
      (if (not (Audio|Components|Audio|IsPlaying (Variables|Character|GetMesh)))
        (Animation|Montage|PlayMontage (Variables|Character|GetMesh) "/Game/Mannequin/Animations/HitReaction/HitReaction_Montage.HitReaction_Montage"
          (:then
            (Development|PrintString (Utilities|String|ToString(Float) (- (Variables|Default|GetCurrentHealth) (+ (Variables|/Game/Assets/Blueprints/Player_Blueprints/ThirdPersonCharacter.ThirdPersonCharacter_C|GetSwordDamage (Variables|Default|GetPlayer)) Damage))))
            (Variables|Default|SetCurrentHealth (- (Variables|Default|GetCurrentHealth) (+ (Variables|/Game/Assets/Blueprints/Player_Blueprints/ThirdPersonCharacter.ThirdPersonCharacter_C|GetSwordDamage (Variables|Default|GetPlayer)) Damage)))
            (Utilities|FlowControl|Delay 0.6)
            (CallFunction|Recovered)))))))

(event EventBeginPlay
  ;[1 1 1] Set inital target to player
  (bind _outactors (Actor|GetAllActorsOfClass "/Game/Assets/Blueprints/Player_Blueprints/ThirdPersonCharacter.ThirdPersonCharacter_C"))
  (Variables|Default|SetPlayer (Utilities|Array|Get(acopy) _outactors))
  ;[1 1 1] Set other values
  (Variables|Default|SetCurrentHealth (Variables|Default|GetMaxHealth))
  (Variables|Default|SetCurrentAttackSpeed (Variables|Default|GetAttackSpeed))
  (bind _asaihealth_bar (Utilities|Casting|CastToAIHealthBar (UserInterface|GetUserWidgetObject (Variables|Default|GetWidget))))
  (Variables|Default|SetHealthbar _asaihealth_bar))

(fn ConstructionScript)

(fn Attack
  (if (< (Variables|Default|GetCurrentAttackSpeed) 0.0)
    (Animation|PlayAnimMontage "/Game/Mannequin/Animations/BruteAttack/BrutePunch_Montage.BrutePunch_Montage" 1.0 "None")
    (bind _asthird_person_character (Utilities|Casting|CastToThirdPersonCharacter (Variables|Default|GetTargetActor))
      (:then
        (Variables|/Game/Assets/Blueprints/Player_Blueprints/ThirdPersonCharacter.ThirdPersonCharacter_C|SetCurrentHealth _asthird_person_character (- (Variables|/Game/Assets/Blueprints/Player_Blueprints/ThirdPersonCharacter.ThirdPersonCharacter_C|GetCurrentHealth _asthird_person_character) (Variables|Default|GetDamage)))
        (Development|PrintString "Player Attacked")
        (Variables|Default|SetCurrentAttackSpeed (Variables|Default|GetAttackSpeed))
        (return))
      (:CastFailed
        (bind _asbp_turret (Utilities|Casting|CastToBP_Turret (Variables|Default|GetTargetActor))
          (:then
            (Variables|/Game/Assets/Blueprints/Turret_Blueprints/BP_Turret.BP_Turret_C|SetCurrentHealth _asbp_turret (- (Variables|/Game/Assets/Blueprints/Turret_Blueprints/BP_Turret.BP_Turret_C|GetCurrentHealth _asbp_turret) (Variables|Default|GetDamage)))
            (Development|PrintString "Turret Attacked")
            (Variables|Default|SetCurrentAttackSpeed (Variables|Default|GetAttackSpeed))
            (return))
          (:CastFailed
            (bind _asdoor_drill (Utilities|Casting|CastToDoor_Drill (Variables|Default|GetTargetActor)))
            (Variables|/Game/Assets/Blueprints/Door_Drll/Door_Drill.Door_Drill_C|SetCurrentHealth _asdoor_drill (- (Variables|/Game/Assets/Blueprints/Door_Drll/Door_Drill.Door_Drill_C|GetCurrentHealth _asdoor_drill) (Variables|Default|GetDamage)))
            (Variables|/Game/Assets/Blueprints/Door_Drll/Door_Drill.Door_Drill_C|SetCurrentRepairTime _asdoor_drill (Variables|/Game/Assets/Blueprints/Door_Drll/Door_Drill.Door_Drill_C|GetRepairTime _asdoor_drill))
            (Development|PrintString "drill attacked")
            (Variables|Default|SetCurrentAttackSpeed (Variables|Default|GetAttackSpeed))))))))

(fn SetTarget
  (if (!= (Variables|Default|GetHealthChange) (Variables|Default|GetCurrentHealth))
    (Variables|Default|SetCurrentChangeTarget 0.0))
  (Variables|Default|SetHealthChange (Variables|Default|GetCurrentHealth))
  (Variables|Default|SetCurrentCheckTarget (- (Variables|Default|GetCurrentCheckTarget) (Utilities|Time|GetWorldDeltaSeconds)))
  (Variables|Default|SetCurrentChangeTarget (- (Variables|Default|GetCurrentChangeTarget) (Utilities|Time|GetWorldDeltaSeconds)))
  (if (and (!= (Variables|Default|GetNewTarget) (Variables|Default|GetTargetActor)) (Utilities|IsValid (Variables|Default|GetNewTarget)))
    ;[1 1 1] When new target is selected
    (if (< (Variables|Default|GetCurrentChangeTarget) 0.0)
      (Variables|Default|SetTargetActor (Variables|Default|GetNewTarget))
      (Variables|Default|SetCurrentChangeTarget (Variables|Default|GetChangeTarget))
      (return)
      (else
        (return)))
    (elif (< (Variables|Default|GetCurrentCheckTarget) 0.0)
      (bind _outactors (Actor|GetAllActorsOfClass "/Game/Assets/Blueprints/Turret_Blueprints/BP_Turret.BP_Turret_C"))
      (for _array_element _outactors
        (if (and (not (LocalVariables|GetCharacterSet)) (< (Math|Vector|Distance(Vector) (Transformation|GetActorLocation self) (Transformation|GetActorLocation _array_element)) (Variables|Default|GetTargetTurretDistance)))
          (Variables|Default|SetNewTarget _array_element)
          (LocalVariables|SetCharacterSet true)
          (Variables|Default|SetCurrentCheckTarget (Variables|Default|GetCheckTarget))
          (return)))
      (if (< (Math|Vector|Distance(Vector) (Transformation|GetActorLocation self) (Transformation|GetActorLocation (Variables|Default|GetPlayer))) (Variables|Default|GetTargetPlayerDistance))
        (Variables|Default|SetNewTarget (Variables|Default|GetPlayer))
        (Variables|Default|SetCurrentCheckTarget (Variables|Default|GetCheckTarget))
        (return)
        (else
          (Utilities|IsValid (Variables|Default|GetDrill)
            (:Is%20Valid
              (if (> (Variables|/Game/Assets/Blueprints/Door_Drll/Door_Drill.Door_Drill_C|GetCurrentHealth (Variables|Default|GetDrill)) 0.0)
                (Variables|Default|SetNewTarget (Variables|Default|GetDrill))
                (Variables|Default|SetCurrentCheckTarget (Variables|Default|GetCheckTarget))
                (return)
                (else
                  _)))
            (:Is%20Not%20Valid
              _))
          (Variables|Default|SetNewTarget (Variables|Default|GetPlayer))
          (Variables|Default|SetCurrentCheckTarget (Variables|Default|GetCheckTarget))
          (return)))
      (else
        (return)))))