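; An enemy spawner actor that periodically spawns a BP_AIEneny1 AI pawn at its own location and rotation.
; Tick counts CurrentTimeToSpawn down by delta time, and once it drops below zero it spawns the pawn and resets the timer to TimeToSpawn.
; The countdown has no spawn limit or activation condition.
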(event EventBeginPlay)

(event Collision|EventActorBeginOverlap
  (params (OtherActor :type Actor%20Object%20Reference)))

(event EventTick
  (params (DeltaSeconds :type Float%20%28single-precision%29))
  (bind _self self)
  (Variables|Default|SetCurrentTimeToSpawn (- (Variables|Default|GetCurrentTimeToSpawn) DeltaSeconds))
  (if (< (Variables|Default|GetCurrentTimeToSpawn) 0.0)
    (AI|SpawnAIFromClass "/Game/Assets/Blueprints/Enemy_Blueprints/BP_AIEneny1.BP_AIEneny1_C" 0 (Transformation|GetActorLocation _self) (Transformation|GetActorRotation _self) false)
    (Variables|Default|SetCurrentTimeToSpawn (Variables|Default|GetTimeToSpawn))))

(fn ConstructionScript)