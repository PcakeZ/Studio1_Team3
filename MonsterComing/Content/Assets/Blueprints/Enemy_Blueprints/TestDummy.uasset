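; Test dummy enemy character that reacts to damage, apparently for trying out hits and weapon knockback.
; On BeginPlay it plays a primary attack animation, freezes it briefly via play rate, then resumes it.
; Damage received while no animation is playing triggers a hit reaction and prints the amount.
; With the player's knockback upgrade, that hit also launches the dummy along the player's negated forward vector, scaled by the GameMode's knockback level.
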(event EventBeginPlay
  (bind _mesh (Variables|Character|GetMesh))
  (Utilities|FlowControl|Delay 2.0)
  (Components|Animation|PlayAnimation _mesh "/Game/Mannequin/Animations/Attack_PrimaryA.Attack_PrimaryA" false)
  (Utilities|FlowControl|Delay 0.2)
  (Components|Timeline|SetPlayRate _mesh 0.0)
  (Utilities|FlowControl|Delay 2.0)
  ;[1 1 1] KNOCKBACK
  (Components|Timeline|SetPlayRate _mesh 1.0))

(event Collision|EventActorBeginOverlap
  (params (OtherActor :type Actor%20Object%20Reference)))

(event EventTick
  (params (DeltaSeconds :type Float%20%28single-precision%29)))

(event Game|Damage|EventAnyDamage
  (params (Damage :type Float%20%28single-precision%29) (DamageType :type Damage%20Type%20Object%20Reference) (InstigatedBy :type Controller%20Object%20Reference) (DamageCauser :type Actor%20Object%20Reference))
  (bind _asthird_person_character (Utilities|Casting|CastToThirdPersonCharacter (Game|GetPlayerCharacter 0)))
  (Variables|Default|SetPlayer%20Reference _asthird_person_character)
  (if (not (Audio|Components|Audio|IsPlaying (Variables|Character|GetMesh)))
    (Components|Animation|PlayAnimation (Variables|Character|GetMesh) "/Game/Mannequin/Animations/HitReaction/HitReaction.HitReaction" false)
    (Development|PrintString (Utilities|String|ToString(Float) Damage))
    (if (Variables|/Game/Assets/Blueprints/Player_Blueprints/ThirdPersonCharacter.ThirdPersonCharacter_C|GetKnockbackUpgrade _asthird_person_character)
      (bind _asthird_person_game_mode (Utilities|Casting|CastToThirdPersonGameMode (Game|GetGameMode)))
      ;[1 1 1] KNOCKBACK
      (Character|LaunchCharacter (* (Math|Vector|NegateVector (Transformation|GetActorForwardVector _asthird_person_character)) (* (Variables|/Game/Assets/Blueprints/GameMode/ThirdPersonGameMode.ThirdPersonGameMode_C|GetWeaponKnockBackLevel _asthird_person_game_mode) 1e+03)) false false))))

(fn ConstructionScript)