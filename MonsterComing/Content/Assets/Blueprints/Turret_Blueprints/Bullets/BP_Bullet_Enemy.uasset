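; BP_Bullet_Enemy is an enemy projectile that damages what it hits and expires after a fixed lifespan.
; On box overlap, a chain of casts subtracts Damage directly from CurrentHealth on the player character, turrets or drill doors, then destroys the bullet.
; Swarm, Recon, Brute and Projectile AI are ignored so the bullet passes through them, while any other actor destroys it.
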(event OnComponentBeginOverlap(Box)
  (params (OverlappedComponent :type Primitive%20Component%20Object%20Reference) (OtherActor :type Actor%20Object%20Reference) (OtherComp :type Primitive%20Component%20Object%20Reference) (OtherBodyIndex :type Integer) (bFromSweep :type Boolean) (SweepResult :type Hit%20Result%20Structure%20%28by%20ref%29))
  (bind _asthird_person_character (Utilities|Casting|CastToThirdPersonCharacter OtherActor)
    (:then
      (Variables|/Game/Assets/Blueprints/Player_Blueprints/ThirdPersonCharacter.ThirdPersonCharacter_C|SetCurrentHealth _asthird_person_character (- (Variables|/Game/Assets/Blueprints/Player_Blueprints/ThirdPersonCharacter.ThirdPersonCharacter_C|GetCurrentHealth _asthird_person_character) (Variables|Default|GetDamage)))
      (Actor|DestroyActor self))
    (:CastFailed
      (bind _asbp_turret (Utilities|Casting|CastToBP_Turret OtherActor)
        (:then
          (Variables|/Game/Assets/Blueprints/Turret_Blueprints/BP_Turret.BP_Turret_C|SetCurrentHealth _asbp_turret (- (Variables|/Game/Assets/Blueprints/Turret_Blueprints/BP_Turret.BP_Turret_C|GetCurrentHealth _asbp_turret) (Variables|Default|GetDamage)))
          (Actor|DestroyActor self))
        (:CastFailed
          (bind _asdoor_drill (Utilities|Casting|CastToDoor_Drill OtherActor)
            (:then
              (Variables|/Game/Assets/Blueprints/Door_Drll/Door_Drill.Door_Drill_C|SetCurrentHealth _asdoor_drill (- (Variables|/Game/Assets/Blueprints/Door_Drll/Door_Drill.Door_Drill_C|GetCurrentHealth _asdoor_drill) (Variables|Default|GetDamage)))
              (Actor|DestroyActor self))
            (:CastFailed
              (Utilities|Casting|CastToBP_AI_Swarm OtherActor
                (:CastFailed
                  (Utilities|Casting|CastToBP_AI_Recon OtherActor
                    (:CastFailed
                      (Utilities|Casting|CastToBP_AI_Brute OtherActor
                        (:CastFailed
                          (Utilities|Casting|CastToBP_AI_Projectile OtherActor
                            (:CastFailed
                              (Actor|DestroyActor self))))))))))))))))

(event EventBeginPlay
  (Actor|SetLifeSpan 1e+01))

(event Collision|EventActorBeginOverlap
  (params (OtherActor :type Actor%20Object%20Reference)))

(event EventTick
  (params (DeltaSeconds :type Float%20%28single-precision%29)))

(fn ConstructionScript)