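; BP_Bullet1 is a turret bullet that damages AI enemies on contact and expires after a fixed lifespan set at BeginPlay.
; Its Box overlap runs a chain of casts over the Swarm, Recon, Brute and Projectile AI types, subtracting Damage directly from CurrentHealth and destroying itself on a match.
; It passes through the player character and turrets, and destroys itself on overlapping anything else.
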(event OnComponentBeginOverlap(Box)
  (params (OverlappedComponent :type Primitive%20Component%20Object%20Reference) (OtherActor :type Actor%20Object%20Reference) (OtherComp :type Primitive%20Component%20Object%20Reference) (OtherBodyIndex :type Integer) (bFromSweep :type Boolean) (SweepResult :type Hit%20Result%20Structure%20%28by%20ref%29))
  ;[1 1 1] Bullet Collides with enemy
  (bind _asbp_ai_swarm (Utilities|Casting|CastToBP_AI_Swarm OtherActor)
    (:then
      (Variables|/Game/Assets/Blueprints/Enemy_Blueprints/BP_AI_Swarm.BP_AI_Swarm_C|SetCurrentHealth _asbp_ai_swarm (- (Variables|/Game/Assets/Blueprints/Enemy_Blueprints/BP_AI_Swarm.BP_AI_Swarm_C|GetCurrentHealth _asbp_ai_swarm) (Variables|Default|GetDamage)))
      (Actor|DestroyActor self))
    (:CastFailed
      ;[1 1 1] Bullet Collides with enemy
      (bind _asbp_ai_recon (Utilities|Casting|CastToBP_AI_Recon OtherActor)
        (:then
          (Variables|/Game/Assets/Blueprints/Enemy_Blueprints/BP_AI_Recon.BP_AI_Recon_C|SetCurrentHealth _asbp_ai_recon (- (Variables|/Game/Assets/Blueprints/Enemy_Blueprints/BP_AI_Recon.BP_AI_Recon_C|GetCurrentHealth _asbp_ai_recon) (Variables|Default|GetDamage)))
          (Actor|DestroyActor self))
        (:CastFailed
          ;[1 1 1] Bullet Collides with enemy
          (bind _asbp_ai_brute (Utilities|Casting|CastToBP_AI_Brute OtherActor)
            (:then
              (Variables|/Game/Assets/Blueprints/Enemy_Blueprints/BP_AI_Brute.BP_AI_Brute_C|SetCurrentHealth _asbp_ai_brute (- (Variables|/Game/Assets/Blueprints/Enemy_Blueprints/BP_AI_Brute.BP_AI_Brute_C|GetCurrentHealth _asbp_ai_brute) (Variables|Default|GetDamage)))
              (Actor|DestroyActor self))
            (:CastFailed
              ;[1 1 1] Bullet Collides with enemy
              (bind _asbp_ai_projectile (Utilities|Casting|CastToBP_AI_Projectile OtherActor)
                (:then
                  (Variables|/Game/Assets/Blueprints/Enemy_Blueprints/BP_AI_Projectile.BP_AI_Projectile_C|SetCurrentHealth _asbp_ai_projectile (- (Variables|/Game/Assets/Blueprints/Enemy_Blueprints/BP_AI_Projectile.BP_AI_Projectile_C|GetCurrentHealth _asbp_ai_projectile) (Variables|Default|GetDamage)))
                  (Actor|DestroyActor self))
                (:CastFailed
                  (Utilities|Casting|CastToThirdPersonCharacter OtherActor
                    (:CastFailed
                      (Utilities|Casting|CastToBP_Turret OtherActor
                        (:CastFailed
                          (Actor|DestroyActor self))))))))))))))

(event EventBeginPlay
  (Actor|SetLifeSpan 1e+01))

(event Collision|EventActorBeginOverlap
  (params (OtherActor :type Actor%20Object%20Reference)))

(event EventTick
  (params (DeltaSeconds :type Float%20%28single-precision%29)))

(fn ConstructionScript)