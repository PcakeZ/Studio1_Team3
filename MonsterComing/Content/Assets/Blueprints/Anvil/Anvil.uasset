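; Anvil actor that upgrades the player's weapon with a knockback ability while the player stands in its overlap area.
; Begin and end overlap cache the ThirdPersonCharacter and toggle its anvil-collision flag, which gates the Upgrade1 event.
; Upgrade1 draws the weapon if needed, spawns an explosion effect, swaps to the second weapon mesh and enables KnockbackUpgrade.
; An inspect montage then plays while movement pauses for a few seconds.
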(event Custom|Upgrade1
  (bind _player_character (Variables|Default|GetPlayer%20Character))
  (bind _player_character_2 (Variables|Default|GetPlayer%20Character))
  (if (Variables|/Game/Assets/Blueprints/Player_Blueprints/ThirdPersonCharacter.ThirdPersonCharacter_C|GetisAnvilColl (stale Collision|EventActorBeginOverlap _output_get))
    (Development|PrintString "upg1")
    ;[1 1 1] sparks come out of anvil
    (if (Variables|/Game/Assets/Blueprints/Player_Blueprints/ThirdPersonCharacter.ThirdPersonCharacter_C|GetWeaponDrawn (stale Collision|EventActorBeginOverlap _output_get))
      (Utilities|FlowControl|Delay 0.2)
      (else
        ;;[1 1 1] equip weapon if not drawn
        (Default|DrawWeapon (stale Collision|EventActorBeginOverlap _output_get))
        (Utilities|FlowControl|Delay 1.3)))
    (Effects|SpawnEmitterAttached "/Game/StarterContent/Particles/P_Explosion.P_Explosion" (Variables|Default|GetParticleSystem) "None" "0, 0, 0" "0, 0, 0" "5.000000,5.000000,5.000000")
    ;[1 1 1] Set upgraded weapon visibility
    (Rendering|SetVisibility (Variables|/Game/Assets/Blueprints/Player_Blueprints/ThirdPersonCharacter.ThirdPersonCharacter_C|GetWeapon _player_character_2) false false)
    (Rendering|SetVisibility (Variables|/Game/Assets/Blueprints/Player_Blueprints/ThirdPersonCharacter.ThirdPersonCharacter_C|GetWeapon2 (Variables|Default|GetPlayer%20Character)) true false)
    ;[1 1 1] Can knockback enemies now
    (Variables|/Game/Assets/Blueprints/Player_Blueprints/ThirdPersonCharacter.ThirdPersonCharacter_C|SetKnockbackUpgrade _player_character_2 true)
    (Animation|Montage|PlayMontage (Variables|/Script/Engine.Character|GetMesh _player_character_2) "/Game/Mannequin/Animations/InspectWeapon_Montage.InspectWeapon_Montage"
      (:then
        ;[1 1 1] Pause movement
        (Variables|/Game/Assets/Blueprints/Player_Blueprints/ThirdPersonCharacter.ThirdPersonCharacter_C|SetCanMove _player_character false)
        (Utilities|FlowControl|Delay 5.0)
        (Variables|/Game/Assets/Blueprints/Player_Blueprints/ThirdPersonCharacter.ThirdPersonCharacter_C|SetCanMove _player_character true)))))

(event Collision|EventActorBeginOverlap
  (params (OtherActor :type Actor%20Object%20Reference))
  (bind _asthird_person_character (Utilities|Casting|CastToThirdPersonCharacter OtherActor))
  (bind _output_get (Variables|Default|SetPlayer%20Character _asthird_person_character))
  (Variables|/Game/Assets/Blueprints/Player_Blueprints/ThirdPersonCharacter.ThirdPersonCharacter_C|SetisAnvilColl _output_get true)
  (Development|PrintString "overlap"))

(event Collision|EventActorEndOverlap
  (params (OtherActor :type Actor%20Object%20Reference))
  (bind _asthird_person_character (Utilities|Casting|CastToThirdPersonCharacter OtherActor))
  (Variables|/Game/Assets/Blueprints/Player_Blueprints/ThirdPersonCharacter.ThirdPersonCharacter_C|SetisAnvilColl _asthird_person_character false)
  (Development|PrintString "not overlap"))

(fn ConstructionScript)