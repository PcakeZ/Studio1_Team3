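; ForwardLevel1 is an endless mode level segment that adds its CreationPoint transform to the Creator's position list when play begins.
; It spawns a drill, resource spawners, enemy spawners and an exit door at component markers, wires them into the drill, and loops over its three phase spawn-delay arrays.
; Overlap triggers reveal and solidify the Back and Front barriers as the player passes.
; Spawned actors are tracked and destroyed with the segment.
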(event OnComponentBeginOverlap(ToggleBack)
  (params (OverlappedComponent :type Primitive%20Component%20Object%20Reference) (OtherActor :type Actor%20Object%20Reference) (OtherComp :type Primitive%20Component%20Object%20Reference) (OtherBodyIndex :type Integer) (bFromSweep :type Boolean) (SweepResult :type Hit%20Result%20Structure%20%28by%20ref%29))
  (bind _back (Variables|Default|GetBack))
  (bind _asthird_person_character (Utilities|Casting|CastToThirdPersonCharacter OtherActor))
  (if (== OtherComp (Variables|/Script/Engine.Character|GetCapsuleComponent _asthird_person_character))
    (Rendering|SetVisibility _back true true)
    (Collision|SetCollisionEnabled _back "QueryAndPhysics")
    (Variables|Default|SetCollided true)))

(event OnComponentEndOverlap(ToggleFront)
  (params (OverlappedComponent :type Primitive%20Component%20Object%20Reference) (OtherActor :type Actor%20Object%20Reference) (OtherComp :type Primitive%20Component%20Object%20Reference) (OtherBodyIndex :type Integer))
  (bind _front (Variables|Default|GetFront))
  (if (Variables|Default|GetCollided)
    (bind _asthird_person_character (Utilities|Casting|CastToThirdPersonCharacter OtherActor))
    (if (== OtherComp (Variables|/Script/Engine.Character|GetCapsuleComponent _asthird_person_character))
      (Rendering|SetVisibility _front true true)
      (Collision|SetCollisionEnabled _front "QueryAndPhysics"))))

(event EventBeginPlay
  (bind _outactors (Actor|GetAllActorsOfClass "/Game/Assets/Blueprints/EndlessModeBlueprints/Creator.Creator_C"))
  (Utilities|Array|Add (Variables|/Game/Assets/Blueprints/EndlessModeBlueprints/Creator.Creator_C|GetPosition (Utilities|Array|Get(acopy) _outactors)) (Transformation|GetWorldTransform (Variables|Default|GetCreationPoint)))
  (bind _returnvalue (Game|SpawnActorfromClass "/Game/Assets/Blueprints/Door_Drll/Door_Drill.Door_Drill_C" (Transformation|GetWorldTransform (Variables|Default|GetDrill)) "Undefined" 0 0))
  (bind _output_get (Variables|Default|SetDoorDrill _returnvalue))
  (Utilities|Array|Add (Variables|Default|GetStuff%20to%20destroy) _output_get)
  (for (_array_element _array_index) (Components|GetChildrenComponents (Variables|Default|GetResourceSpawner) false)
    (bind _returnvalue_2 (Game|SpawnActorfromClass "/Game/Assets/Blueprints/Resource_BluePrints/BP_ResourceSpawner.BP_ResourceSpawner_C" (Transformation|GetWorldTransform _array_element) "Undefined" 0 0))
    (Utilities|Array|Add (Variables|/Game/Assets/Blueprints/Door_Drll/Door_Drill.Door_Drill_C|GetResourceSpawners (Variables|Default|GetDoorDrill)) _returnvalue_2)
    (Utilities|Array|Add (Variables|Default|GetStuff%20to%20destroy) _returnvalue_2)
    (if (== _array_index 0)
      (Variables|/Game/Assets/Blueprints/Resource_BluePrints/BP_ResourceSpawner.BP_ResourceSpawner_C|SetResourceActive _returnvalue_2 true)))
  (for _array_element_2 (Components|GetChildrenComponents (Variables|Default|GetEnemySpawnPoints) false)
    (bind _returnvalue_3 (Game|SpawnActorfromClass "/Game/Assets/Blueprints/Enemy_Blueprints/BP_EnemySpawner.BP_EnemySpawner_C" (Transformation|GetWorldTransform _array_element_2) "Undefined" 0 0))
    (Utilities|Array|Add (Variables|/Game/Assets/Blueprints/Door_Drll/Door_Drill.Door_Drill_C|GetSpawnpointArray (Variables|Default|GetDoorDrill)) _returnvalue_3)
    (Utilities|Array|Add (Variables|Default|GetStuff%20to%20destroy) _returnvalue_3))
  (bind _returnvalue_4 (Game|SpawnActorfromClass "/Game/Assets/Blueprints/EndlessModeBlueprints/DoorEndless.DoorEndless_C" (Transformation|GetWorldTransform (Variables|Default|GetDoor)) "Undefined" 0 0))
  (Variables|/Game/Assets/Blueprints/Door_Drll/Door_Drill.Door_Drill_C|SetEndlessDoor (Variables|Default|GetDoorDrill) _returnvalue_4)
  (Utilities|Array|Add (Variables|Default|GetStuff%20to%20destroy) _returnvalue_4)
  (Collision|SetCollisionEnabled (Variables|Default|GetBack) "NoCollision")
  (Collision|SetCollisionEnabled (Variables|Default|GetFront) "NoCollision")
  ;[1 1 1] Set up Phases
  (for _array_element_3 (Variables|/Game/Assets/Blueprints/Door_Drll/Door_Drill.Door_Drill_C|GetPhase1Spawndelay (Variables|Default|GetDoorDrill))
    (Utilities|Array|SetArrayElem (Variables|/Game/Assets/Blueprints/Door_Drll/Door_Drill.Door_Drill_C|GetPhase1Spawndelay (Variables|Default|GetDoorDrill)) 0 0.0))
  (for _array_element_4 (Variables|/Game/Assets/Blueprints/Door_Drll/Door_Drill.Door_Drill_C|GetPhase2Spawndelay (Variables|Default|GetDoorDrill))
    (Utilities|Array|SetArrayElem (Variables|/Game/Assets/Blueprints/Door_Drll/Door_Drill.Door_Drill_C|GetPhase2Spawndelay (Variables|Default|GetDoorDrill)) 0 0.0))
  (for _array_element_5 (Variables|/Game/Assets/Blueprints/Door_Drll/Door_Drill.Door_Drill_C|GetPhase3Spawndelay (Variables|Default|GetDoorDrill))
    (Utilities|Array|SetArrayElem (Variables|/Game/Assets/Blueprints/Door_Drll/Door_Drill.Door_Drill_C|GetPhase3Spawndelay (Variables|Default|GetDoorDrill)) 0 0.0)))

(event EventDestroyed
  (for _array_element (Variables|Default|GetStuff%20to%20destroy)
    (Actor|DestroyActor _array_element)))

(event EventTick
  (params (DeltaSeconds :type Float%20%28single-precision%29)))

(fn ConstructionScript)