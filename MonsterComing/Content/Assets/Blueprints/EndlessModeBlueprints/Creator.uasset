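; Creator procedurally builds an endless-mode level from forward, left and right room pieces, one step per Tick.
; Each step spawns a random piece at the last Position transform, an array this graph only reads and trims.
; A distance check against used positions detects overlap, replacing the last room with a random piece and counting failures.
; At the room or failure limit, it swaps the last room for EndLevel.
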(event EventBeginPlay)

(event Collision|EventActorBeginOverlap
  (params (OtherActor :type Actor%20Object%20Reference)))

(event EventTick
  (params (DeltaSeconds :type Float%20%28single-precision%29))
  (if (not (Variables|Default|GetRoomsBuilt))
    (CallFunction|CreateStuff)))

(fn ConstructionScript)

(fn CreateStuff
  (bind _allrooms (Variables|Default|GetAllRooms))
  (bind _usedpositions (Variables|Default|GetUsedPositions))
  (bind _position (Variables|Default|GetPosition))
  (bind _position_2 (Variables|Default|GetPosition))
  (bind _position_3 (Variables|Default|GetPosition))
  (bind _position_4 (Variables|Default|GetPosition))
  (bind _allrooms_2 (Variables|Default|GetAllRooms))
  (bind _usedpositions_2 (Variables|Default|GetUsedPositions))
  (bind _position_5 (Variables|Default|GetPosition))
  (bind _position_6 (Variables|Default|GetPosition))
  (bind _returnvalue (Utilities|Array|Length _allrooms))
  (bind _returnvalue_2 (Utilities|Array|Length _allrooms_2))
  (bind _returnvalue_3 (- _returnvalue 1))
  (bind _returnvalue_4 (- _returnvalue_2 1))
  (if (< (Variables|Default|GetCurrentRoom) (Variables|Default|GetMaxRooms))
    (Development|PrintString (Utilities|String|ToString(Integer) (Variables|Default|GetCurrentRoom)))
    (if (== (Variables|Default|GetCurrentRoom) 0)
      (bind _returnvalue_5 (Game|SpawnActorfromClass "/Game/Assets/Blueprints/EndlessModeBlueprints/ForwardLevel1.ForwardLevel1_C" (Math|Transform|MakeTransform "0, 0, 0" "0, 0, 0" "1,1,1") "Undefined" 0 0))
      (Utilities|Array|Add (Variables|Default|GetAllRooms) _returnvalue_5)
      (Utilities|Array|Add (Variables|Default|GetUsedPositions) (Transformation|GetActorLocation _returnvalue_5))
      (Math|Integer|IncrementInt (Variables|Default|GetCurrentRoom))
      (else
        (CallFunction|TestOverlap)
        (if (Variables|Default|GetOverlap)
          (if (< (Variables|Default|GetFailCount) (Variables|Default|GetMaxFailCount))
            (Math|Integer|IncrementInt (Variables|Default|GetFailCount)
              (:%20%20
                (Actor|DestroyActor (Utilities|Array|Get(acopy) _allrooms_2 _returnvalue_4))
                (Utilities|Array|RemoveIndex _allrooms_2 _returnvalue_4)
                (Utilities|Array|RemoveIndex _usedpositions_2 (- (Utilities|Array|Length _usedpositions_2) 1))
                (Utilities|Array|RemoveIndex _position_5 (- (Utilities|Array|Length _position_5) 1))
                (Math|Integer|DecrementInt (Variables|Default|GetCurrentRoom)
                  (:%20%20
                    (switch int (Math|Random|RandomIntegerinRange 0 2) :!label _label
                      (:0
                        ;[1 1 1] Left
                        (switch int (Math|Random|RandomIntegerinRange 0 0)
                          (:0
                            (bind _returnvalue_6 (Game|SpawnActorfromClass "/Game/Assets/Blueprints/EndlessModeBlueprints/LeftLevel.LeftLevel_C" (Utilities|Array|Get(acopy) _position_4 (- (Utilities|Array|Length _position_4) 1)) "Undefined" 0 0))
                            (Utilities|Array|Add (Variables|Default|GetAllRooms) _returnvalue_6)
                            (Utilities|Array|Add (Variables|Default|GetUsedPositions) (Transformation|GetActorLocation _returnvalue_6))
                            (Math|Integer|IncrementInt (Variables|Default|GetCurrentRoom)))))
                      (:1
                        ;[1 1 1] Forward
                        (switch int (Math|Random|RandomIntegerinRange 0 0) :!label _label_2
                          (:0
                            (bind _returnvalue_7 (Game|SpawnActorfromClass "/Game/Assets/Blueprints/EndlessModeBlueprints/ForwardLevel1.ForwardLevel1_C" (Utilities|Array|Get(acopy) _position_2 (- (Utilities|Array|Length _position_2) 1)) "Undefined" 0 0))
                            (Utilities|Array|Add (Variables|Default|GetAllRooms) _returnvalue_7)
                            (Utilities|Array|Add (Variables|Default|GetUsedPositions) (Transformation|GetActorLocation _returnvalue_7))
                            (Math|Integer|IncrementInt (Variables|Default|GetCurrentRoom)))))
                      (:2
                        ;[1 1 1] Right
                        (switch int (Math|Random|RandomIntegerinRange 0 0)
                          (:0
                            (bind _returnvalue_8 (Game|SpawnActorfromClass "/Game/Assets/Blueprints/EndlessModeBlueprints/RightLevel.RightLevel_C" (Utilities|Array|Get(acopy) _position_6 (- (Utilities|Array|Length _position_6) 1)) "Undefined" 0 0))
                            (Utilities|Array|Add (Variables|Default|GetAllRooms) _returnvalue_8)
                            (Utilities|Array|Add (Variables|Default|GetUsedPositions) (Transformation|GetActorLocation _returnvalue_8))
                            (Math|Integer|IncrementInt (Variables|Default|GetCurrentRoom)))))
                      (:3
                        (goto _label_2)))))))
            (else
              (Variables|Default|SetRoomsBuilt true)
              (Actor|DestroyActor (Utilities|Array|Get(acopy) _allrooms _returnvalue_3) :!label _label_3)
              (Utilities|Array|RemoveIndex _allrooms _returnvalue_3)
              (Utilities|Array|RemoveIndex _usedpositions (- (Utilities|Array|Length _usedpositions) 1))
              (Utilities|Array|RemoveIndex _position_3 (- (Utilities|Array|Length _position_3) 1))
              ;[1 1 1] EndRoom
              (switch int (Math|Random|RandomIntegerinRange 0 0)
                (:0
                  (bind _returnvalue_9 (Game|SpawnActorfromClass "/Game/Assets/Blueprints/EndlessModeBlueprints/EndLevel.EndLevel_C" (Utilities|Array|Get(acopy) _position (- (Utilities|Array|Length _position) 1)) "Undefined" 0 0))
                  (Utilities|Array|Add (Variables|Default|GetAllRooms) _returnvalue_9)
                  (Utilities|Array|Add (Variables|Default|GetUsedPositions) (Transformation|GetActorLocation _returnvalue_9))))))
          (else
            (Variables|Default|SetFailCount 0)
            (goto _label)))))
    (else
      (Variables|Default|SetRoomsBuilt true)
      (goto _label_3))))

(fn TestOverlap
  (bind _position (Variables|Default|GetPosition))
  (Variables|Default|SetOverlap false)
  (for _array_element (Variables|Default|GetUsedPositions)
    (if (not (Variables|Default|GetOverlap))
      (if (< (Math|Vector|Distance(Vector) _array_element (.location (Utilities|Array|Get(acopy) _position (- (Utilities|Array|Length _position) 1)))) 5e+02)
        (Variables|Default|SetOverlap true)
        (return))))
  (return))