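; EndLevel is an Endless Mode level piece that registers its CreationPoint transform with the Creator actor on BeginPlay.
; When the player's capsule overlaps ToggleBack, the Back component becomes visible and solid, and Collided is set.
; On destruction it also destroys everything tracked in StuffToDestroy.
; Disconnected logic would spawn resource spawners for DoorDrill and randomize its phase-one delays by room progress and difficulty, but never runs.
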(event OnComponentBeginOverlap(ToggleBack)
  (params (OverlappedComponent :type Primitive%20Component%20Object%20Reference) (OtherActor :type Actor%20Object%20Reference) (OtherComp :type Primitive%20Component%20Object%20Reference) (OtherBodyIndex :type Integer) (bFromSweep :type Boolean) (SweepResult :type Hit%20Result%20Structure%20%28by%20ref%29))
  (bind _back (Variables|Default|GetBack))
  (bind _asthird_person_character (Utilities|Casting|CastToThirdPersonCharacter OtherActor))
  (if (== OtherComp (Variables|/Script/Engine.Character|GetCapsuleComponent _asthird_person_character))
    (Rendering|SetVisibility _back true false)
    (Collision|SetCollisionEnabled _back "QueryAndPhysics")
    (Variables|Default|SetCollided true)))

(event EventBeginPlay
  (bind _outactors (Actor|GetAllActorsOfClass "/Game/Assets/Blueprints/EndlessModeBlueprints/Creator.Creator_C"))
  (Utilities|Array|Add (Variables|/Game/Assets/Blueprints/EndlessModeBlueprints/Creator.Creator_C|GetPosition (Utilities|Array|Get(acopy) _outactors)) (Transformation|GetWorldTransform (Variables|Default|GetCreationPoint))))

(event EventDestroyed
  (for _array_element (Variables|Default|GetStuff%20to%20destroy)
    (Actor|DestroyActor _array_element)))

(event EventTick
  (params (DeltaSeconds :type Float%20%28single-precision%29)))

(fn ConstructionScript)