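; Healing station actor that restores the player's health from a limited pool while the player is in range and below full health.
; Tick caches the player character, runs a range check and sets CanInteract on the game mode, while the TestDistance event toggles healing.
; A Delay inside Tick paces health transfer into fixed steps.
; The point light shows active healing, then stays red once the pool empties.
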(event Custom|TestDistance
  (Variables|Default|SetHealingPlayer (not (Variables|Default|GetHealingPlayer))))

(event EventBeginPlay
  (Variables|Default|SethealingRange 2e+04)
  (Variables|Default|SethealthPerSecond 1e+01)
  (bind _output_get (Variables|Default|SetmaxHealing 1e+02))
  (Variables|Default|SetcurrentHealing _output_get))

(event Collision|EventActorBeginOverlap
  (params (OtherActor :type Actor%20Object%20Reference)))

(event EventTick
  (params (DeltaSeconds :type Float%20%28single-precision%29))
  (bind _healthpersecond (Variables|Default|GethealthPerSecond))
  (bind _pointlight (Variables|Default|GetPointLight))
  (bind _returnvalue (* _healthpersecond 0.2))
  (if (> (Variables|Default|GetcurrentHealing) 0.0)
    (Rendering|SetVisibility (Variables|Default|GetPointLight) (Variables|Default|GetHealingPlayer) false)
    (Utilities|IsValid (Variables|Default|GetPlayer)
      (:Is%20Valid
        (Class|HealingStation|TestPlayerDistance)
        (if (and (Variables|Default|GetinRange) (< (Variables|/Game/Assets/Blueprints/Player_Blueprints/ThirdPersonCharacter.ThirdPersonCharacter_C|GetCurrentHealth (Variables|Default|GetPlayer)) 1e+02))
          (bind _asthird_person_game_mode (Utilities|Casting|CastToThirdPersonGameMode (Game|GetGameMode)))
          (Variables|/Game/Assets/Blueprints/GameMode/ThirdPersonGameMode.ThirdPersonGameMode_C|SetCanInteract _asthird_person_game_mode true)
          (if (Variables|Default|GetHealingPlayer)
            (Utilities|FlowControl|Delay 0.2)
            (Variables|/Game/Assets/Blueprints/Player_Blueprints/ThirdPersonCharacter.ThirdPersonCharacter_C|SetCurrentHealth (Variables|Default|GetPlayer) (+ (Variables|/Game/Assets/Blueprints/Player_Blueprints/ThirdPersonCharacter.ThirdPersonCharacter_C|GetCurrentHealth (Variables|Default|GetPlayer)) _returnvalue))
            (Variables|Default|SetcurrentHealing (- (Variables|Default|GetcurrentHealing) _returnvalue)))
          (else
            (Variables|Default|SetHealingPlayer false))))
      (:Is%20Not%20Valid
        (bind _asthird_person_character (Utilities|Casting|CastToThirdPersonCharacter (Game|GetPlayerCharacter 0)))
        (Variables|Default|SetPlayer _asthird_person_character)))
    (else
      (Rendering|SetVisibility _pointlight true false)
      (Rendering|Components|Light|SetLightColor _pointlight "(R=1.000000,G=0.000000,B=0.000000,A=1.000000)" true))))

(fn ConstructionScript)