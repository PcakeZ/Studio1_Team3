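; Drill trigger actor that runs a timed three-phase enemy wave event, with a placement preview shown while the player overlaps its box.
; Start reveals the drill and activates only its assigned resource spawners.
; Tick counts down per-phase delay arrays: slot zero advances the phase, while other slots spawn matching enemy classes at random spawnpoints.
; TimerFinished deactivates resource spawners, zeroes enemy health, spawns an enemy at a fixed location and destroys the actor.
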(event EventBeginPlay
  (bind _phase1spawndelay (Variables|Default|GetPhase1Spawndelay))
  ;[1 1 1] Set inital visibility
  (Rendering|SetVisibility (Variables|Default|GetDrillStuff) false true)
  (Rendering|SetVisibility (Variables|Default|GetCube5) false true)
  ;[1 1 1] Set start time and phase 1
  (Variables|Default|SetCurrentSpawndelay _phase1spawndelay)
  (bind _output_get (Variables|Default|SetStartTime (+ (Utilities|Array|Get(acopy) (Variables|Default|GetPhase3Spawndelay)) (+ (Utilities|Array|Get(acopy) (Variables|Default|GetPhase2Spawndelay)) (Utilities|Array|Get(acopy) _phase1spawndelay)))))
  (Variables|Default|SetTimeRemaining _output_get))

(event Collision|EventActorBeginOverlap
  (params (OtherActor :type Actor%20Object%20Reference)))

(event EventTick
  (params (DeltaSeconds :type Float%20%28single-precision%29))
  (bind _cube5 (Variables|Default|GetCube5))
  (bind _spawnpointarray (Variables|Default|GetSpawnpointArray))
  (bind _returnvalue (Utilities|Array|Length _spawnpointarray))
  (bind _returnvalue_2 (- _returnvalue 1))
  (bind _returnvalue_3 (Math|Random|RandomIntegerinRange 0 _returnvalue_2))
  (bind _output (Utilities|Array|Get(acopy) _spawnpointarray _returnvalue_3))
  (if (Variables|Default|GetIsActive)
    ;[1 1 1] Set Timers
    (Variables|Default|SetTimeRemaining (- (Variables|Default|GetTimeRemaining) (Utilities|Time|GetWorldDeltaSeconds)))
    (for (_array_element _array_index) (Variables|Default|GetCurrentSpawndelay)
      ;[1 1 1] Subtract deltatime from value
      (Utilities|Array|SetArrayElem (Variables|Default|GetCurrentSpawndelay) _array_index (- _array_element (Utilities|Time|GetWorldDeltaSeconds)))
      ;[1 1 1] Test if time is up
      (if (<= _array_element 0.0)
        (if (== _array_index 0)
          ;[1 1 1] Next Phase
          (switch int (Variables|Default|GetCurrentPhase)
            (:1
              (Variables|Default|SetCurrentSpawndelay (Variables|Default|GetPhase2Spawndelay))
              (Math|Integer|IncrementInt (Variables|Default|GetCurrentPhase)))
            (:2
              (Variables|Default|SetCurrentSpawndelay (Variables|Default|GetPhase3Spawndelay))
              (Math|Integer|IncrementInt (Variables|Default|GetCurrentPhase)))
            (:3
              ;[1 1 1] All phases completed
              (CallFunction|TimerFinished)))
          (else
            ;[1 1 1] Spawn enemy
            (AI|SpawnAIFromClass (Utilities|GetClass (Utilities|Array|Get(acopy) (Variables|Default|GetEnemyArray) (- _array_index 1))) 0 (Transformation|GetActorLocation _output) (Transformation|GetActorRotation _output) false)
            ;[1 1 1] Rest timer based on phase
            (switch int (Variables|Default|GetCurrentPhase)
              (:1
                (Utilities|Array|SetArrayElem (Variables|Default|GetCurrentSpawndelay) _array_index (Utilities|Array|Get(acopy) (Variables|Default|GetPhase1Spawndelay) _array_index)))
              (:2
                (Utilities|Array|SetArrayElem (Variables|Default|GetCurrentSpawndelay) _array_index (Utilities|Array|Get(acopy) (Variables|Default|GetPhase2Spawndelay) _array_index)))
              (:3
                (Utilities|Array|SetArrayElem (Variables|Default|GetCurrentSpawndelay) _array_index (Utilities|Array|Get(acopy) (Variables|Default|GetPhase3Spawndelay) _array_index))))))))
    (else
      ;[1 1 1] Set drilling placer visibility
      (if (> (Utilities|Array|Length (Collision|GetOverlappingActors (Variables|Default|GetBox) "/Game/Assets/Blueprints/Player_Blueprints/ThirdPersonCharacter.ThirdPersonCharacter_C" :!class /Script/Engine.PrimitiveComponent)) 0)
        (Rendering|SetVisibility _cube5 true true)
        (else
          (Rendering|SetVisibility _cube5 false true))))))

(fn ConstructionScript)

(fn TimerFinished
  ;[1 1 1] Set resource spawner values
  (bind _outactors (Actor|GetAllActorsOfClass "/Game/Assets/Blueprints/Resource_BluePrints/BP_ResourceSpawner.BP_ResourceSpawner_C"))
  (for _array_element _outactors
    (Variables|/Game/Assets/Blueprints/Resource_BluePrints/BP_ResourceSpawner.BP_ResourceSpawner_C|SetSpawnerActive _array_element false)
    ;[1 1 1] Kill all Enemies
    (bind _outactors_2 (Actor|GetAllActorsOfClass "/Game/Assets/Blueprints/Enemy_Blueprints/BP_AIEneny1.BP_AIEneny1_C"))
    (for (_array_element_2 _array_index) _outactors_2
      (if (>= _array_index (- (Utilities|Array|Length _outactors_2) 1))
        (AI|SpawnAIFromClass "/Game/Assets/Blueprints/Enemy_Blueprints/BP_AIEneny1.BP_AIEneny1_C" 0 "-1131.002563,-3280.000000,226.001602" "0, 0, 0" false)
        (Variables|/Game/Assets/Blueprints/Enemy_Blueprints/BP_AIEneny1.BP_AIEneny1_C|SetCurrentHealth _array_element_2 0.0)
        (else
          (Variables|/Game/Assets/Blueprints/Enemy_Blueprints/BP_AIEneny1.BP_AIEneny1_C|SetCurrentHealth _array_element_2 0.0))))
    (AI|SpawnAIFromClass "/Game/Assets/Blueprints/Enemy_Blueprints/BP_AIEneny1.BP_AIEneny1_C" 0 "-1131.002563,-3280.000000,226.001602" "0, 0, 0" false)
    (Actor|DestroyActor)))

(fn Start
  (if (not (Variables|Default|GetIsActive))
    ;[1 1 1] Set drill visibility
    (Rendering|SetVisibility (Variables|Default|GetDrillStuff) true true)
    (Rendering|SetVisibility (Variables|Default|GetCube5) false true)
    (Variables|Default|SetIsActive true)
    ;[1 1 1] Set up resource spawners
    (bind _outactors (Actor|GetAllActorsOfClass "/Game/Assets/Blueprints/Resource_BluePrints/BP_ResourceSpawner.BP_ResourceSpawner_C"))
    (for _array_element _outactors
      (Variables|/Game/Assets/Blueprints/Resource_BluePrints/BP_ResourceSpawner.BP_ResourceSpawner_C|SetSpawnerActive _array_element false))
    (for _array_element_2 (Variables|Default|GetResourceSpawners)
      (Variables|/Game/Assets/Blueprints/Resource_BluePrints/BP_ResourceSpawner.BP_ResourceSpawner_C|SetSpawnerActive _array_element_2 true))))