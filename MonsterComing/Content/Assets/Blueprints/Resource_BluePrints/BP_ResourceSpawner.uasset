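; BP_ResourceSpawner is a spawn point that shows a collectible resource and credits the player when it is collected.
; Tick shows the resource while spawner and resource are active; otherwise an active spawner's timer can activate a random active spawner's resource.
; ResourceSpawned stops that timer until CollectResource resets it on the same spawner and increments the player's ResourcesCollected.
; AllActiveArray accumulates candidates without being cleared.
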(event EventBeginPlay
  (bind _outactors (Actor|GetAllActorsOfClass "/Game/Assets/Blueprints/Player_Blueprints/ThirdPersonCharacter.ThirdPersonCharacter_C"))
  (Variables|Default|SetPlayer (Utilities|Array|Get(acopy) _outactors)))

(event Collision|EventActorBeginOverlap
  (params (OtherActor :type Actor%20Object%20Reference)))

(event EventTick
  (params (DeltaSeconds :type Float%20%28single-precision%29))
  (bind _allactivearray (Variables|Default|GetAllActiveArray))
  (bind _resource (Variables|Default|GetResource))
  ;[0.02567 1 0.9003] Test if resource is active
  (if (Variables|Default|GetSpawnerActive)
    (if (Variables|Default|GetResourceActive)
      ;[1 1 1] Set resource visibility
      (Rendering|SetVisibility _resource true true)
      (else
        (Rendering|SetVisibility _resource false true)
        (if (not (Variables|Default|GetResourceSpawned))
          (Variables|Default|SetCurrentSpawnTimer (- (Variables|Default|GetCurrentSpawnTimer) DeltaSeconds))
          (if (<= (Variables|Default|GetCurrentSpawnTimer) 0.0)
            (bind _outactors (Actor|GetAllActorsOfClass "BP_ResourceSpawner_C"))
            (for _array_element _outactors
              ;[1 0 0.5966] Check if spawners are active
              (if (Variables|BP_ResourceSpawner_C|GetSpawnerActive _array_element)
                (Utilities|Array|Add (Variables|Default|GetAllActiveArray) _array_element)))
            ;[0.1169 1 0] Set values
            (Variables|BP_ResourceSpawner_C|SetResourceActive (Utilities|Array|Get(acopy) _allactivearray (Math|Random|RandomIntegerinRange 0 (- (Utilities|Array|Length _allactivearray) 1))) true)
            (Variables|Default|SetCurrentSpawnTimer (Variables|Default|GetResourceSpawnTimer))
            (Variables|Default|SetResourceSpawned true)
            (Development|PrintString "Resource Spawned")))))
    (else
      (Rendering|SetVisibility (Variables|Default|GetResource) false true))))

(event Collision|EventActorEndOverlap
  (params (OtherActor :type Actor%20Object%20Reference)))

(fn ConstructionScript)

(fn CollectResource
  (bind _player (Variables|Default|GetPlayer))
  ;[1 1 1] Test then rest values
  (if (Variables|Default|GetSpawnerActive)
    (if (Variables|Default|GetResourceActive)
      (Variables|Default|SetResourceActive false)
      (Variables|Default|SetResourceSpawned false)
      (Variables|/Game/Assets/Blueprints/Player_Blueprints/ThirdPersonCharacter.ThirdPersonCharacter_C|SetResourcesCollected _player (+ (Variables|/Game/Assets/Blueprints/Player_Blueprints/ThirdPersonCharacter.ThirdPersonCharacter_C|GetResourcesCollected _player) 1))
      (Development|PrintString "Resource Collected"))))