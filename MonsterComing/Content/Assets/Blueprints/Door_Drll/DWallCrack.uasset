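; DWallCrack is a wall crack actor for the drillable door that stays hidden until the player starts drilling.
; On BeginPlay it hides itself and caches the player's ThirdPersonCharacter.
; Tick polls that character's StartDrilling flag and reveals the crack once through a DoOnce.
; A HideCrack event hides it again, with no reset of the DoOnce in this graph.
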(event Custom|Hide%20Crack
  (Rendering|SetActorHiddenInGame true))

(event EventBeginPlay
  (Rendering|SetActorHiddenInGame true)
  (bind _asthird_person_character (Utilities|Casting|CastToThirdPersonCharacter (Game|Player|GetPlayerPawn 0)))
  (Variables|Default|SetTPCRef _asthird_person_character))

(event EventTick
  (params (DeltaSeconds :type Float%20%28single-precision%29))
  (if (Variables|/Game/Assets/Blueprints/Player_Blueprints/ThirdPersonCharacter.ThirdPersonCharacter_C|GetStartDrilling (Variables|Default|GetTPCRef))
    (Utilities|FlowControl|DoOnce false
      (:Completed
        (Rendering|SetActorHiddenInGame false)))))

(fn ConstructionScript)